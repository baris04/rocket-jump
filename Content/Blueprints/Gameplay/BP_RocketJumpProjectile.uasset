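; BP_RocketJumpProjectile is a projectile that launches the player away from its impact point for rocket jumping.
; When ProjectileMovement stops, it checks whether player character 0 is within ExplosionRadius, then destroys itself either way.
; A player in range gets a fixed-strength LaunchCharacter along the normalized direction away from the projectile, biased upward, overriding existing velocity.
; The sphere overlap and mesh hit events are empty.
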(event `self.Sphere.OnComponentBeginOverlap`
  (params (OverlappedComponent :type "PrimitiveComponent Object Reference") (OtherActor :type "Actor Object Reference") (OtherComp :type "PrimitiveComponent Object Reference") (OtherBodyIndex :type Integer) (bFromSweep :type Boolean) (SweepResult :type "HitResult Structure (by ref)")))

(event `self.StaticMesh.OnComponentHit`
  (params (HitComponent :type "PrimitiveComponent Object Reference") (OtherActor :type "Actor Object Reference") (OtherComp :type "PrimitiveComponent Object Reference") (NormalImpulse :type "Vector Structure") (Hit :type "HitResult Structure (by ref)")))

(event `self.ProjectileMovement.OnProjectileStop`
  (params (ImpactResult :type "HitResult Structure (by ref)"))
  (bind _returnvalue (`GameplayStatics.GetPlayerCharacter` 0))
  (if (<= (`KismetMathLibrary.Vector_Distance` (`self.K2_GetActorLocation` (`GameplayStatics.GetPlayerCharacter` 0)) (`self.K2_GetActorLocation`)) (`self.Explosion Radius`))
    (`Character.LaunchCharacter` _returnvalue (* (`KismetMathLibrary.Normal` (+ (`KismetMathLibrary.Normal` (- (`self.K2_GetActorLocation` _returnvalue) (`self.K2_GetActorLocation`))) (0.0 0.0 0.45))) 1000.0) true true))
  (`self.K2_DestroyActor`))

(fn `UserConstructionScript`)